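; Game mode for what appears to be a lane-based runner, handling track tiles, rocks and the game flow.
; On BeginPlay it caches the game state and chains initial BP_Chank tiles, each placed at the previous one's SpawnPoint.
; Start, End and Restart forward to the game state, with End also clearing rocks.
; SpawnRock picks one of three lanes with random scale; its event-graph call and the difficulty increase are unwired.
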(event Custom|Process
  (params (CurrentTime :type Integer))
  (if (== (Math|Integer|%(Integer) CurrentTime (Variables|Default|GetIncreaseDifficultyTime)) 0)
    _))

(event Custom|End
  (Default|EndGameEvent (Variables|Default|GetAs%20BP%20Game%20State))
  (Utilities|DestroyAllRocks))

(event Custom|RestartGame
  (Default|RestartGameEvent (Variables|Default|GetAs%20BP%20Game%20State)))

(event Custom|StartGame
  (Default|StartGameEvent (Variables|Default|GetAs%20BP%20Game%20State)))

(event EventBeginPlay
  (Utilities|Initialize)
  (for _index (range 0 1)
    (CallFunction|SpawnTile)))

(fn ConstructionScript)

(fn SpawnRock
  (switch int (Math|Random|RandomInteger 3)
    (:0
      (Game|SpawnActorfromClass "/Game/MyGame/Blueprints/BP_Rock.BP_Rock_C" (Math|Transform|MakeTransform (Math|Vector|MakeVector 1.3e+02 3.5e+03 4e+01) "0, 0, 0" (Math|Conversions|ToVector(Float) (Math|Random|RandomFloatinRange 1.0 2.0))) "AdjustIfPossibleButAlwaysSpawn" "MultiplyWithRoot" 0 0))
    (:1
      (Game|SpawnActorfromClass "/Game/MyGame/Blueprints/BP_Rock.BP_Rock_C" (Math|Transform|MakeTransform (Math|Vector|MakeVector 5.8e+02 3.5e+03 4e+01) "0, 0, 0" (Math|Conversions|ToVector(Float) (Math|Random|RandomFloatinRange 1.0 2.0))) "AdjustIfPossibleButAlwaysSpawn" "MultiplyWithRoot" 0 0))
    (:2
      (Game|SpawnActorfromClass "/Game/MyGame/Blueprints/BP_Rock.BP_Rock_C" (Math|Transform|MakeTransform (Math|Vector|MakeVector 9.7e+02 3.5e+03 4e+01) "0, 0, 0" (Math|Conversions|ToVector(Float) (Math|Random|RandomFloatinRange 1.0 2.0))) "AdjustIfPossibleButAlwaysSpawn" "MultiplyWithRoot" 0 0))))

(fn GetMaxDeathCount
  (return (Variables|Default|GetMaxDeathCount)))

(fn SpawnTile
  (bind _returnvalue (Game|SpawnActorfromClass "/Game/MyGame/Blueprints/BP_Chank.BP_Chank_C" (Variables|Default|GetSpawn%20Transform) "Undefined" "MultiplyWithRoot" 0 0))
  (bind _asbp_chank (Utilities|Casting|CastToBP_Chank _returnvalue))
  (Variables|Default|SetSpawn%20Transform (Math|Transform|MakeTransform (Transformation|GetWorldLocation (Variables|/Game/MyGame/Blueprints/BP_Chank.BP_Chank_C|GetSpawnPoint _asbp_chank)) "0.000000,0.000000,0.000000" "1.000000,1.000000,1.000000")))