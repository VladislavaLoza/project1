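; BP_Rock is a hazard actor that moves along negative world Y at Speed and kills the player on contact.
; BeginPlay caches the game state, player pawn and game mode.
; While the round is running, a capsule overlap with BP_Character destroys both actors and calls End on the game mode.
; DestroyWithDelay explodes the rock after a random delay; the turning and bounce helpers are left unconnected.
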(event OnComponentBeginOverlap(Capsule)
  (params (OverlappedComponent :type Primitive%20Component%20Object%20Reference) (OtherActor :type Actor%20Object%20Reference) (OtherComp :type Primitive%20Component%20Object%20Reference) (OtherBodyIndex :type Integer) (bFromSweep :type Boolean) (SweepResult :type Hit%20Result%20Structure%20%28by%20ref%29))
  ;[1 1 1] Удаление игрока при столкновении
  (if (not (Default|GetRoundEnded (Variables|Default|GetAs%20BP%20Game%20State)))
    (bind _asbp_character (Utilities|Casting|CastToBP_Character OtherActor))
    (Actor|DestroyActor _asbp_character)
    (Actor|DestroyActor)
    (Default|End (Variables|Default|GetAs%20BP%20Game%20Mode))))

(event Custom|DestroyWithDelay
  ;[1 1 1] События удаления объекта
  (Utilities|FlowControl|Delay (Math|Random|RandomFloatinRange 0.5 2.0))
  (Effects|SpawnEmitteratLocation "/Game/StarterContent/Particles/P_Explosion.P_Explosion" (Transformation|GetActorLocation))
  (Actor|DestroyActor))

(event EventBeginPlay
  ;[1 1 1] Начало игры
  (|Обновлениеверхнегоменю))

(event EventTick
  (params (DeltaSeconds :type Float%20%28single-precision%29))
  (bind _returnvalue (Transformation|GetActorLocation))
  ;[1 1 1] Смещение объекта
  (Transformation|SetActorLocation (Math|Vector|MakeVector (.x _returnvalue) (- (.y _returnvalue) (* DeltaSeconds (Variables|Default|GetSpeed))) (.z _returnvalue)) false false))

(event Collision|EventHit
  (params (MyComp :type Primitive%20Component%20Object%20Reference) (Other :type Actor%20Object%20Reference) (OtherComp :type Primitive%20Component%20Object%20Reference) (bSelfMoved :type Boolean) (HitLocation :type Vector :default "0, 0, 0") (HitNormal :type Vector :default "0, 0, 0") (NormalImpulse :type Vector :default "0, 0, 0") (Hit :type Hit%20Result%20Structure%20%28by%20ref%29)))

(fn ConstructionScript)