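; Player controller that owns the HUD widget and links its start, restart and exit requests to the game.
; On possess it creates WBP_HUD, adds it to the viewport and binds to its three events.
; Start and restart switch to game-only input with a hidden cursor before calling BP_GameMode, while exit quits the game.
; BeginPlay enables game-and-UI input with a visible cursor, and GetWidget exposes the HUD.
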(event Custom|OnRestartGame_Event
  (CallFunction|ActivateGameMode)
  (bind _asbp_game_mode (Utilities|Casting|CastToBP_GameMode (Game|GetGameMode)))
  (Default|RestartGame _asbp_game_mode))

(event Custom|QuitEvent
  (Game|QuitGame 0 "Quit" false))

(event Custom|OnStartGame_Event
  (CallFunction|ActivateGameMode)
  (bind _asbp_game_mode (Utilities|Casting|CastToBP_GameMode (Game|GetGameMode)))
  (Default|StartGame _asbp_game_mode))

(event EventPossess
  (params (PossessedPawn :type Pawn%20Object%20Reference))
  (bind _returnvalue (UserInterface|CreateWidget "/Game/MyGame/Blueprints/WBP_HUD.WBP_HUD_C" self))
  (UserInterface|Viewport|AddtoViewport _returnvalue 0)
  (bind _output_get (Variables|Default|SetHUDWdget _returnvalue))
  (EventDispatchers|AssignOnStartGame _output_get (delegate Custom|OnStartGame_Event))
  (EventDispatchers|BindEventtoOnRestartGame _output_get (delegate Custom|OnRestartGame_Event))
  (EventDispatchers|BindEventtoOnExitGame _output_get (delegate Custom|QuitEvent)))

(event EventBeginPlay
  (CallFunction|ActivateUIMode))

(fn ConstructionScript)

(fn GetWidget
  (return (Variables|Default|GetHUDWdget)))

(fn ActivateUIMode
  (Input|SetInputModeGameandUI self (Variables|Default|GetHUDWdget) "DoNotLock" true false)
  (Variables|Default|SetbShowMouseCursor true))

(fn ActivateGameMode
  (Input|SetInputModeGameOnly self false)
  (Variables|Default|SetbShowMouseCursor false))