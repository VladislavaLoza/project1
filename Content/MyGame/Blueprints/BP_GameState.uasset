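; Game state for a score-and-lives game, tracking play time, difficulty (shown as rocks on the HUD) and round/game-over flags.
; A looping one-second timer passes elapsed time to BP_GameMode and refreshes the HUD through the player controller's widget.
; Ending stores high score and deaths in BP_GameInstance, then shows round end or game over by death limit.
; Restart reloads the level, clearing both records after game over.
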(event Custom|StartGameEvent
  (bind _returnvalue (Utilities|Time|SetTimerbyEvent (delegate Custom|MainTimerEvent) 1.0 true))
  (Variables|Default|SetTimer _returnvalue)
  (Variables|Default|SetIsRoundEnded false)
  (Variables|Default|SetIsGameEnded false))

(event Custom|MainTimerEvent
  (Math|Integer|IncrementInt (Variables|Default|GetTimePlayed)
    (:%20%20
      (Default|Process (Variables|Default|GetAs%20BP%20Game%20Mode) (Variables|Default|GetTimePlayed))
      (Utilities|UpdateHUD))))

(event Custom|EndGameEvent
  (bind _as_bp_game_instance (Variables|Default|GetAs%20BP%20Game%20Instance))
  (Utilities|Time|ClearandInvalidateTimerbyHandle (Variables|Default|GetTimer))
  (Default|UpdateHighestScore _as_bp_game_instance (Default|GetPlayerScore (Variables|Default|GetAs%20BP%20Player%20State)))
  (Default|IncreaseDeathCount _as_bp_game_instance)
  (Default|ActivateUIMode (Variables|Default|GetAs%20BP%20Player%20Controller))
  (Utilities|UpdateHUD)
  (if (CallFunction|IsGameOverCondition)
    (Variables|Default|SetIsGameEnded true)
    (bind _hud (Default|GetWidget (Variables|Default|GetAs%20BP%20Player%20Controller)))
    (Default|GameOver _hud)
    (else
      (Variables|Default|SetIsRoundEnded true)
      (bind _hud_2 (Default|GetWidget (Variables|Default|GetAs%20BP%20Player%20Controller)))
      (Default|EndGame _hud_2)
      (Default|UpdateLives _hud_2 (- (Default|GetMaxDeathCount (Variables|Default|GetAs%20BP%20Game%20Mode)) (Default|GetDeathCount (Variables|Default|GetAs%20BP%20Game%20Instance)))))))

(event Custom|RestartGameEvent
  (bind _as_bp_game_instance (Variables|Default|GetAs%20BP%20Game%20Instance))
  (bind _returnvalue (Game|GetCurrentLevelName true))
  (Game|OpenLevel(byName) (Utilities|String|StringToName _returnvalue))
  ;[1 1 1] After Game Over
  (if (CallFunction|IsGameOverCondition)
    (Default|ClearDeathCount _as_bp_game_instance)
    (Default|ClearHigestScore _as_bp_game_instance)))

(event EventBeginPlay
  (Utilities|Initialize)
  (Utilities|UpdateHUD))

(fn ConstructionScript)

(fn GetTimePlayed
  (return (Variables|Default|GetTimePlayed)))

(fn GetDifficulty
  (return (Variables|Default|GetDifficulty)))

(fn GetRoundEnded
  (return (Variables|Default|GetIsRoundEnded)))

(fn GetGameEnded
  (return (Variables|Default|GetIsGameEnded)))

(fn InreaseDifficulty
  (Variables|Default|SetDifficulty (+ (Variables|Default|GetDifficulty) 1)))

(fn IsGameOverCondition
  (return (>= (Default|GetDeathCount (Variables|Default|GetAs%20BP%20Game%20Instance)) (Default|GetMaxDeathCount (Variables|Default|GetAs%20BP%20Game%20Mode)))))