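; BP_Destroy is a moving actor that destroys rocks it touches and awards a point for each.
; Tick moves it along the world Y axis at Speed, scaled by delta time.
; An overlap with a BP_Rock destroys the rock and increments the score stored in BP_GameMode.
; The new score goes to two HUD text fields, reached through game state and player controller references chained from the game mode.
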(event OnComponentBeginOverlap(CollisionComponent)
  (params (OverlappedComponent :type Primitive%20Component%20Object%20Reference) (OtherActor :type Actor%20Object%20Reference) (OtherComp :type Primitive%20Component%20Object%20Reference) (OtherBodyIndex :type Integer) (bFromSweep :type Boolean) (SweepResult :type Hit%20Result%20Structure%20%28by%20ref%29))
  (bind _asbp_rock (Utilities|Casting|CastToBP_Rock OtherActor))
  (Actor|DestroyActor _asbp_rock)
  (bind _asbp_game_mode (Utilities|Casting|CastToBP_GameMode (Game|GetGameMode)))
  (bind _output_get (Variables|/Game/MyGame/Blueprints/BP_GameMode.BP_GameMode_C|SetScorre _asbp_game_mode (+ (Variables|/Game/MyGame/Blueprints/BP_GameMode.BP_GameMode_C|GetScorre _asbp_game_mode) 1)))
  (Rendering|Components|TextRender|SetText (Variables|/Game/MyGame/Blueprints/WBP_HUD.WBP_HUD_C|GetScore (Variables|/Game/MyGame/Blueprints/BP_PlayerController.BP_PlayerController_C|GetHUDWdget (Variables|/Game/MyGame/Blueprints/BP_GameState.BP_GameState_C|GetAs%20BP%20Player%20Controller (Variables|/Game/MyGame/Blueprints/BP_GameMode.BP_GameMode_C|GetAs%20BP%20Game%20State _asbp_game_mode)))) (Utilities|Text|ToText(Integer) _output_get))
  (Rendering|Components|TextRender|SetText (Variables|/Game/MyGame/Blueprints/WBP_HUD.WBP_HUD_C|GetScore_1 (Variables|/Game/MyGame/Blueprints/BP_PlayerController.BP_PlayerController_C|GetHUDWdget (Variables|/Game/MyGame/Blueprints/BP_GameState.BP_GameState_C|GetAs%20BP%20Player%20Controller (Variables|/Game/MyGame/Blueprints/BP_GameMode.BP_GameMode_C|GetAs%20BP%20Game%20State _asbp_game_mode)))) (Utilities|Text|ToText(Integer) _output_get)))

(event EventTick
  (params (DeltaSeconds :type Float%20%28single-precision%29))
  (bind _returnvalue (Transformation|GetActorLocation))
  (Transformation|SetActorLocation (Math|Vector|MakeVector (.x _returnvalue) (+ (.y _returnvalue) (* DeltaSeconds (Variables|Default|GetSpeed))) (.z _returnvalue)) false false))

(event EventBeginPlay)

(fn ConstructionScript)