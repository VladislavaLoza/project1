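; BP_Chank is a level chunk that asks BP_GameMode to spawn the next tile when BP_Character enters its Trigger.
; Tick feeds a random Delay of a few seconds, acting as a repeating timer for the Спавн камня (rock spawn) graph.
; That graph spawns a BP_Rock at a random point inside the Zone box.
; The delayed self-destroy logic is disconnected, so the chunk never destroys itself here.
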(event OnComponentBeginOverlap(Trigger)
  (params (OverlappedComponent :type Primitive%20Component%20Object%20Reference) (OtherActor :type Actor%20Object%20Reference) (OtherComp :type Primitive%20Component%20Object%20Reference) (OtherBodyIndex :type Integer) (bFromSweep :type Boolean) (SweepResult :type Hit%20Result%20Structure%20%28by%20ref%29))
  (Utilities|Casting|CastToBP_Character OtherActor)
  (bind _asbp_game_mode (Utilities|Casting|CastToBP_GameMode (Game|GetGameMode)))
  (Default|SpawnTile _asbp_game_mode))

(event OnComponentEndOverlap(zone)
  (params (OverlappedComponent :type Primitive%20Component%20Object%20Reference) (OtherActor :type Actor%20Object%20Reference) (OtherComp :type Primitive%20Component%20Object%20Reference) (OtherBodyIndex :type Integer)))

(event EventBeginPlay)

(event EventTick
  (params (DeltaSeconds :type Float%20%28single-precision%29))
  (Utilities|FlowControl|Delay (Math|Random|RandomFloatinRange 2.0 4.0))
  (if true
    (|Спавнкамня)))

(fn ConstructionScript)